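; BP_DMK_LeashActor is a leash anchor actor that becomes active while the player pawn is inside its sphere trigger.
; Sphere overlap events toggle IsActive and cache or clear the player's controller.
; GetLeashOriginLocation exposes the Target component's world location as the leash origin; the Blueprint's graphs apply no leash movement or constraint themselves.
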(event `self.Sphere.OnComponentBeginOverlap`
  (params (OverlappedComponent :type "PrimitiveComponent Object Reference") (OtherActor :type "Actor Object Reference") (OtherComp :type "PrimitiveComponent Object Reference") (OtherBodyIndex :type Integer) (bFromSweep :type Boolean) (SweepResult :type "HitResult Structure (by ref)"))
  (bind _returnvalue (`GameplayStatics.GetPlayerPawn` 0))
  (if (== OtherActor _returnvalue)
    (set `self.bIsActive` true)
    (bind _asplayer_controller (cast `PlayerController` (`Pawn.GetController` _returnvalue)))
    (set `self.CachedPlayerController` _asplayer_controller)))

(event `self.Sphere.OnComponentEndOverlap`
  (params (OverlappedComponent :type "PrimitiveComponent Object Reference") (OtherActor :type "Actor Object Reference") (OtherComp :type "PrimitiveComponent Object Reference") (OtherBodyIndex :type Integer))
  (if (== OtherActor (`GameplayStatics.GetPlayerPawn` 0))
    (set `self.bIsActive` false)
    (set `self.CachedPlayerController` null)))

(fn `GetLeashOriginLocation`
  (returns (ReturnValue :type "Vector Structure"))
  (return (`SceneComponent.K2_GetComponentLocation` (`self.Target`))))

(fn `UserConstructionScript`)